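; Building actor that shakes around its starting location when ShakeBuilding is called with a magnitude, frequency and duration.
; Tick offsets the actor with out-of-phase sine and cosine waves per axis, with weaker vertical motion, then snaps it back once the duration ends.
; Amplitude eases toward the requested magnitude by a fixed per-frame lerp, so the ramp is frame-rate dependent and carries over between shakes.
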(event `self.ReceiveBeginPlay`
  (set `self.DefaultLocation` (`self.K2_GetActorLocation`)))

(event `ShakeBuilding`
  (params (Magnitude :type "Float (double-precision)") (Frequency :type "Float (double-precision)") (Duration :type "Float (double-precision)"))
  (set `self.IsShaking` true)
  (set `self.ShakeMagnitude` Magnitude)
  (set `self.ShakeFrequency` Frequency)
  (set `self.ShakeDuration` Duration)
  (set `self.ShakeTimer` 0.0))

(event `self.ReceiveTick`
  (params (DeltaSeconds :type "Float (single-precision)"))
  (if (`self.IsShaking`)
    (set `self.Lerp ShakeMagnitude` (`KismetMathLibrary.Lerp` (`self.Lerp ShakeMagnitude`) (`self.ShakeMagnitude`) 0.01))
    (bind _output_get (set `self.ShakeTimer` (+ (`self.ShakeTimer`) DeltaSeconds)))
    (`self.K2_SetActorLocation` (+ (`KismetMathLibrary.MakeVector` (* (* (`KismetMathLibrary.Sin` (* (* _output_get (`self.ShakeFrequency`)) 10.0)) (`self.Lerp ShakeMagnitude`)) 10.0) (* (* (`KismetMathLibrary.Cos` (* (* _output_get (`self.ShakeFrequency`)) 8.0)) (`self.Lerp ShakeMagnitude`)) 10.0) (* (* (`KismetMathLibrary.Sin` (* (* _output_get (`self.ShakeFrequency`)) 6.0)) (`self.Lerp ShakeMagnitude`)) 5.0)) (`self.DefaultLocation`)))
    (if (>= (`self.ShakeTimer`) (`self.ShakeDuration`))
      (`self.K2_SetActorLocation` (`self.DefaultLocation`))
      (set `self.IsShaking` false))))

(fn `UserConstructionScript`)