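; Manager that stages a scripted earthquake shortly after BeginPlay, with camera shake, scream sounds and a rumble.
; StartEarthquake sphere-overlaps around an origin and passes magnitude, frequency and duration to each ShakableBuilding_BP found.
; School desks simulate physics until the quake's timed end; the rumble pauses on its own timer and UnPausedSound resumes it.
; Tick eases LerpMagnitude toward Magnitude, but the shake does not use that value.
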(event `UnPausedSound`
  (`AudioComponent.SetPaused` (stale `self.ReceiveBeginPlay` _returnvalue) false))

(event `self.ReceiveBeginPlay`
  (`KismetSystemLibrary.Delay` 0.5)
  (`self.SetPhysics Object` true)
  (`KismetSystemLibrary.Delay` 0.5)
  (`KismetSystemLibrary.Delay` 3.0)
  (`|ExecutionSequence`
    (:`then_0`
      (`self.StartEarthquake`)
      (`KismetSystemLibrary.Delay` 9.0)
      (`self.SetPhysics Object` false))
    (:`then_1`
      (set `self.StartEQ` true))
    (:`then_2`
      (`PlayerCameraManager.StartCameraShake` :`self` (`GameplayStatics.GetPlayerCameraManager` 0) :`ShakeClass` "/Script/Engine.CameraShakeBase")
      (`|ExecutionSequence`
        (:`then_0`
          (`GameplayStatics.PlaySound2D` "/Game/Petch/Sounds/female-scream.female-scream" 1.0 1.0 0.0 null null)
          (`GameplayStatics.PlaySound2D` "/Game/Petch/Sounds/female-scream-longer.female-scream-longer" 1.0 1.0 0.0 null null)
          (`GameplayStatics.PlaySound2D` "/Game/Petch/Sounds/female-scream-short.female-scream-short" 1.0 1.0 0.0 null null))
        (:`then_1`
          (bind _returnvalue (`GameplayStatics.CreateSound2D` "/Game/Petch/Sounds/Earthquake_sound_effect.Earthquake_sound_effect" 1.0 1.0 0.0 null))
          (`AudioComponent.Play` _returnvalue 0.0)
          (`KismetSystemLibrary.Delay` 6.0)
          (`AudioComponent.SetPaused` _returnvalue true))))))

(event `self.ReceiveTick`
  (params (DeltaSeconds :type "Float (single-precision)"))
  (if (`self.StartEQ`)
    (bind _output_get (set `self.Lerp Magnitude` (`KismetMathLibrary.Lerp` (`self.Lerp Magnitude`) (`self.Magnitude`) 0.01)))))

(event `StartEarthquake`
  (bind _outactors (`KismetSystemLibrary.SphereOverlapActors` (`self.Origin`) (`self.Radius`) (`self.Object Types`)))
  (for _array_element _outactors
    (bind _asshakable_building_bp (cast `/Game/Nice/Blueprints/ShakableBuilding_BP` _array_element))
    (`/Game/Nice/Blueprints/ShakableBuilding_BP.ShakeBuilding` _asshakable_building_bp (`self.Magnitude`) (`self.Frequancy`) (`self.Duration`))))

(event `SetPhysics Object`
  (params (Simulate :type Boolean))
  (bind _outactors (`GameplayStatics.GetAllActorsOfClass` "/Game/Asset/3DModel/Desk/source/SchoolDesk_Blueprint.SchoolDesk_Blueprint_C"))
  (for _array_element _outactors
    (`PrimitiveComponent.SetSimulatePhysics` (`StaticMeshActor.StaticMeshComponent` _array_element) Simulate)))

(fn `UserConstructionScript`)