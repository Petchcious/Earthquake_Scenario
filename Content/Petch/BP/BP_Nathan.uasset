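; BP_Nathan is an injured character in a VR first-aid interaction, with events for pain, hurt and looping-state injured audio.
; Tick raises a clamped AidPercent while his hand is held and the pawn grabs, draining it otherwise until the teacher step.
; Near full aid, BP_Bandage gets an outline and can be applied through the Box overlap.
; Applying it destroys the bandage, reveals the call-teacher widget and switches the player's dialogue page.
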(event `PlayPainSound`
  (`GameplayStatics.PlaySound2D` "/Game/Petch/Sounds/man-in-sudden-pain.man-in-sudden-pain" 1.0 1.0 0.0 null null)
  (`KismetSystemLibrary.Delay` 1.3)
  (`GameplayStatics.PlaySound2D` "/Game/Petch/Sounds/man-in-sudden-pain2.man-in-sudden-pain2" 1.0 1.0 0.0 null null))

(event `StopInjuredSound`
  (`AudioComponent.Stop` (`self.InjuredSound`)))

(event `self.ReceiveBeginPlay`
  (`SceneComponent.SetVisibility` (`self.Aid`) false false)
  (`SceneComponent.SetVisibility` (`self.GlowingArm`) false false)
  (bind _aspetch_vrpawn_1 (cast `/Game/Petch/Petch_VRPawn1` (`GameplayStatics.GetPlayerCharacter` 0)))
  (set `self.As Petch VRPawn 1` _aspetch_vrpawn_1))

(event `PlayInjuredSound`
  (`self.InjuredSound`
    (:`then`
      _)
    (:`else`
      (bind _returnvalue (`GameplayStatics.CreateSound2D` "/Game/Petch/Sounds/Injured.Injured" 1.0 1.0 0.0 null))
      (set `self.InjuredSound` _returnvalue)))
  (`AudioComponent.Play` (`self.InjuredSound`) 0.0))

(event `PlayHurtSound`
  (`self.HurtSound`
    (:`then`
      _)
    (:`else`
      (bind _returnvalue (`GameplayStatics.CreateSound2D` "/Game/Petch/Sounds/Hurt.Hurt" 1.0 1.0 0.0 null))
      (set `self.HurtSound` _returnvalue)))
  (`AudioComponent.SetPaused` (`self.InjuredSound`) true)
  (`AudioComponent.Play` (`self.HurtSound`) 0.0)
  (`KismetSystemLibrary.Delay` 1.0)
  (`AudioComponent.SetPaused` (`self.InjuredSound`) false))

(event `AddAid`
  (if (`self.IsHandHold`)
    (if (`/Game/Petch/Petch_VRPawn1.IsGrab?` (`self.As Petch VRPawn 1`))
      (`/Engine/EditorBlueprintResources/StandardMacros.DoOnce` false :!label _label
        (:`Completed`
          (set `self.AidPercent` (`KismetMathLibrary.Lerp` (`self.AidPercent`) (+ (`self.AidPercent`) 5.0) 0.5))
          (`KismetSystemLibrary.Delay` 0.1)
          (goto _label :!via `Reset`))))))

(event `self.ReceiveTick`
  (params (DeltaSeconds :type "Float (single-precision)"))
  (`|ExecutionSequence`
    (:`then_0`
      (if (`self.IsHandHold`)
        (`self.AddAid`)
        (elif (not (`self.ShowTeacherUI`))
          (`/Engine/EditorBlueprintResources/StandardMacros.DoOnce` false :!label _label_2
            (:`Completed`
              (set `self.AidPercent` (`KismetMathLibrary.Lerp` (`self.AidPercent`) (+ (`self.AidPercent`) -2.5) 0.5))
              (`KismetSystemLibrary.Delay` 0.1)
              (goto _label_2 :!via `Reset`))))))
    (:`then_1`
      (if (>= (`self.AidPercent`) 95.0)
        (set `self.CanBandage?` true)
        (bind _outactors (`GameplayStatics.GetAllActorsOfClass` "/Game/Petch/BP/BP_Bandage.BP_Bandage_C"))
        (bind _output (`|GetArrayItem` _outactors))
        (`/Engine/EditorBlueprintResources/StandardMacros.IsValid` _output
          (:`Is Valid`
            (bind _staticmeshcomponent (`StaticMeshActor.StaticMeshComponent` _output))
            (`MeshComponent.SetOverlayMaterial` _staticmeshcomponent "/Game/Petch/Mats/M_Outline_Inst.M_Outline_Inst")
            (`SceneComponent.SetVisibility` _staticmeshcomponent true false)))
        (else
          (set `self.CanBandage?` false)
          (bind _outactors_2 (`GameplayStatics.GetAllActorsOfClass` "/Game/Petch/BP/BP_Bandage.BP_Bandage_C"))
          (bind _output_2 (`|GetArrayItem` _outactors_2))
          (`/Engine/EditorBlueprintResources/StandardMacros.IsValid` _output_2
            (:`Is Valid`
              (`MeshComponent.SetOverlayMaterial` (`StaticMeshActor.StaticMeshComponent` _output_2) "/Game/Petch/Assets/Mat/01_-_Default.01_-_Default"))))))
    (:`then_2`
      (if (`self.ShowTeacherUI`)
        (`/Engine/EditorBlueprintResources/StandardMacros.DoOnce` false
          (:`Completed`
            (bind _outactors_3 (`GameplayStatics.GetAllActorsOfClass` "/Game/Petch/BP/BP_CallTeacher.BP_CallTeacher_C"))
            (`SceneComponent.SetVisibility` (`/Game/Petch/BP/BP_CallTeacher.Widget` (`|GetArrayItem` _outactors_3)) true false)
            (bind _aspetch_vrpawn_1 (cast `/Game/Petch/Petch_VRPawn1` (`GameplayStatics.GetPlayerPawn` 0)))
            (bind _aswbp_choice_first_aid (cast `/Game/Petch/Widgets/WBP_Choice_FirstAid` (`WidgetComponent.GetWidget` (`/Game/Petch/Petch_VRPawn1.DialougeWidget` _aspetch_vrpawn_1))))
            (`/Game/Petch/Widgets/WBP_Choice_FirstAid.ChangeWidgetIndex` _aswbp_choice_first_aid 1)))))
    (:`then_3`
      (if (<= (`self.AidPercent`) 0.0)
        (set `self.AidPercent` 0.0)))
    (:`then_4`
      (if (>= (`self.AidPercent`) 100.0)
        (set `self.AidPercent` 100.0)))))

(event `self.Box.OnComponentBeginOverlap`
  (params (OverlappedComponent :type "PrimitiveComponent Object Reference") (OtherActor :type "Actor Object Reference") (OtherComp :type "PrimitiveComponent Object Reference") (OtherBodyIndex :type Integer) (bFromSweep :type Boolean) (SweepResult :type "HitResult Structure (by ref)"))
  (if (`self.CanBandage?`)
    (bind _asbp_bandage (cast `/Game/Petch/BP/BP_Bandage` OtherActor))
    (`self.K2_DestroyActor` _asbp_bandage)
    (set `self.ShowTeacherUI` true)))

(event `self.Box.OnComponentEndOverlap`
  (params (OverlappedComponent :type "PrimitiveComponent Object Reference") (OtherActor :type "Actor Object Reference") (OtherComp :type "PrimitiveComponent Object Reference") (OtherBodyIndex :type Integer)))

(fn `UserConstructionScript`)