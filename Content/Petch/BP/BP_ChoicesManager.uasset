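; BP_ChoicesManager times the earthquake choice prompt and slows the game when it appears.
; On BeginPlay it hides the first BP_Choices_Earthquake widget, reveals it after a delay, then sets a very low global time dilation.
; StopTimeDilation plays a timeline whose updates restore normal speed and overwrite the PostProcessVolume settings.
; A second post-process settings branch is left unconnected.
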(event `StartTime Dilation`
  (`GameplayStatics.SetGlobalTimeDilation` 0.05))

(event `self.ReceiveBeginPlay`
  (bind _outactors (`GameplayStatics.GetAllActorsOfClass` "/Game/Petch/BP/BP_Choices_Earthquake.BP_Choices_Earthquake_C"))
  (bind _widget (`/Game/Petch/BP/BP_Choices_Earthquake.Widget` (`|GetArrayItem` _outactors)))
  (`SceneComponent.SetVisibility` _widget false false)
  (`KismetSystemLibrary.Delay` 10.0)
  (`SceneComponent.SetVisibility` _widget true false)
  (`KismetSystemLibrary.Delay` 0.2)
  (`self.StartTime Dilation`))

(event `StopTime Dilation`
  (`|ExecutionSequence`
    (:`then_0`
      (`Timeline|Timeline` :!via `PlayFromStart`
        (:`Update`
          (`GameplayStatics.SetGlobalTimeDilation` 1.0)
          (bind _returnvalue (`GameplayStatics.GetActorOfClass` "/Script/Engine.PostProcessVolume"))
          (set `PostProcessVolume.Settings` (make `PostProcessSettings`) _returnvalue))))))

(fn `UserConstructionScript`)